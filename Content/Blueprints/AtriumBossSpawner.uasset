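; Level actor that spawns the atrium boss when the campaign reaches the right point.
; On BeginPlay it reads MyGame, the game instance, and acts only if the key card is held and CampaignState is 1.
; SpawnBoss then spawns BossBP with its behavior tree at the actor's root, ignoring collision, and adds the boss health bar widget to the viewport.
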(event `self.ReceiveBeginPlay`
  (bind _asmy_game (cast `/Game/Blueprints/MyGame` (`GameplayStatics.GetGameInstance`)))
  (if (and (`/Game/Blueprints/MyGame.hasKeyCard` _asmy_game) (== (`/Game/Blueprints/MyGame.campaignState` _asmy_game) 1))
    (`self.spawnBoss`)))

(fn `spawnBoss`
  (`KismetSystemLibrary.PrintString` "spawned boss")
  (`AIBlueprintHelperLibrary.SpawnAIFromClass` "/Game/Blueprints/BossBP.BossBP_C" "/Game/Blueprints/EnemyAIBase/BossBT.BossBT" (`SceneComponent.K2_GetComponentLocation` (`self.DefaultSceneRoot`)) (struct) true null)
  (bind _returnvalue (`|CreateWidget` "/Game/Widget/bossHealthBarWBP.bossHealthBarWBP_C"))
  (`UserWidget.AddToViewport` _returnvalue 0))

(fn `UserConstructionScript`)