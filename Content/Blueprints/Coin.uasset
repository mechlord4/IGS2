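; Coin pickup that flies to the player and adds to their coin count.
; On overlap with the player's FirstPersonCharacter, the Attract timeline moves Sphere1 toward the character's live position.
; Each update lerps from the sphere's current location, so the pull compounds and tracks a moving player.
; When the timeline finishes, it passes CoinAmount to AddCoins and destroys itself.
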(event `self.ReceiveActorBeginOverlap`
  (params (OtherActor :type "Actor Object Reference"))
  (if (== OtherActor (`GameplayStatics.GetPlayerCharacter` 0))
    (bind _asfirst_person_character (cast `/Game/FirstPersonBP/Blueprints/FirstPersonCharacter` OtherActor))
    (bind (_direction _distance__normalized_) (`Timeline|Attract`)
      (:`Update`
        (`SceneComponent.K2_SetWorldLocation` (`self.Sphere1`) (`KismetMathLibrary.VLerp` (`SceneComponent.K2_GetComponentLocation` (`self.Sphere1`)) (`SceneComponent.K2_GetComponentLocation` (`Actor.RootComponent` _asfirst_person_character)) _distance__normalized_) false false))
      (:`Finished`
        (`/Game/FirstPersonBP/Blueprints/FirstPersonCharacter.addCoins` _asfirst_person_character (`self.coinAmount`))
        (`self.K2_DestroyActor`)))))

(fn `UserConstructionScript`)