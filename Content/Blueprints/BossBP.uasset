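; Boss enemy that fires projectiles from two barrels and drops loot on death.
; Tick and damage events feed blackboard keys for player proximity and LowHealth, the latter set on any hit.
; At zero health it awards score, clears the player's BossAlive flag and spawns paint chips, coins, random pickups and attachments.
; GameInstance multipliers scale chips and coins, while nested rolls pick attachment rarity.
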(event `self.ReceiveBeginPlay`
  (bind _asfirst_person_character (cast `/Game/FirstPersonBP/Blueprints/FirstPersonCharacter` (`GameplayStatics.GetPlayerCharacter` 0)))
  (set `/Game/FirstPersonBP/Blueprints/FirstPersonCharacter.bossAlive` true _asfirst_person_character)
  (set `/Game/FirstPersonBP/Blueprints/FirstPersonCharacter.bossBPReference` self _asfirst_person_character)
  (bind _asmy_game (cast `/Game/Blueprints/MyGame` (`GameplayStatics.GetGameInstance`)))
  (set `self.As My Game` _asmy_game))

(event `self.ReceiveTick`
  (params (DeltaSeconds :type "Float (single-precision)"))
  (bind _returnvalue (`AIBlueprintHelperLibrary.GetBlackboard` (`AIBlueprintHelperLibrary.GetAIController` self)))
  (if (<= (`KismetMathLibrary.Vector_Distance` (`SceneComponent.K2_GetComponentLocation` (`self.RootComponent`)) (`SceneComponent.K2_GetComponentLocation` (`Actor.RootComponent` (`GameplayStatics.GetPlayerCharacter` 0)))) 2500.0)
    (`BlackboardComponent.SetValueAsBool` _returnvalue "CloseToPlayer" true)
    (else
      (`BlackboardComponent.SetValueAsBool` _returnvalue "CloseToPlayer" false))))

(event `self.ReceiveAnyDamage`
  (params (Damage :type "Float (single-precision)") (DamageType :type "DamageType Object Reference") (InstigatedBy :type "Controller Object Reference") (DamageCauser :type "Actor Object Reference"))
  (`AISense_Damage.ReportDamageEvent` self DamageCauser Damage)
  (bind _output_get (set `self.Health` (- (`self.Health`) Damage)))
  (if true
    (`BlackboardComponent.SetValueAsBool` (`AIBlueprintHelperLibrary.GetBlackboard` null) "LowHealth" true)
    (if (<= _output_get 0.0)
      (`self.Drop Pick Up`)
      (bind _asfirst_person_character (cast `/Game/FirstPersonBP/Blueprints/FirstPersonCharacter` (`GameplayStatics.GetPlayerCharacter` 0)))
      (`/Game/FirstPersonBP/Blueprints/FirstPersonCharacter.addScore` _asfirst_person_character 3)
      (`/Game/FirstPersonBP/Blueprints/FirstPersonCharacter.addEndlessEnemiesKilled` _asfirst_person_character)
      (set `/Game/FirstPersonBP/Blueprints/FirstPersonCharacter.bossAlive` false _asfirst_person_character)
      (`self.K2_DestroyActor`))))

(event `chargeUpNoise`
  (`KismetSystemLibrary.PrintString` "Hello")
  (`GameplayStatics.PlaySoundAtLocation` "/Game/Assets/bossChargeSound.bossChargeSound" (`SceneComponent.K2_GetComponentLocation` (`self.StaticMesh`)) (struct) 0.2 1.0 0.0 "/Game/Blueprints/BossProjAttennuation.BossProjAttennuation" null null))

(fn `ChargeNoise`
  (`GameplayStatics.PlaySoundAtLocation` "/Game/StarterContent/Audio/Light01.Light01" (`SceneComponent.K2_GetComponentLocation` (`self.StaticMesh`)) (struct) 1.0 1.0 0.0 null null null))

(fn `Drop Pick Up`
  (bind _returnvalue (`KismetMathLibrary.RandomFloatInRange` 0.0 100.0))
  (bind _currentchips (`self.currentChips`))
  (bind _counter (`self.counter`))
  (bind _returnvalue_2 (`SceneComponent.K2_GetComponentLocation` (`self.CapsuleComponent`)))
  (bind _returnvalue_3 (`KismetMathLibrary.MakeRotator` 0.0 0.0 (`KismetMathLibrary.RandomFloatInRange` 0.0 360.0)))
  (bind _returnvalue_4 (`KismetMathLibrary.MakeTransform` _returnvalue_2 _returnvalue_3 (0.2 0.2 0.2)))
  (`|ExecutionSequence`
    (:`then_0`
      ;[1 1 1] Spawn Paintchips
      (bind _output_get (set `self.currentChips` (`KismetMathLibrary.RandomIntegerInRange` 20 40)))
      (bind _asmy_game (cast `/Game/Blueprints/MyGame` (`GameplayStatics.GetGameInstance`)))
      (bind _luckmulti (`/Game/Blueprints/MyGame.getLuckMulti` _asmy_game))
      (`|SpawnActorFromClass` "/Game/Blueprints/paintChip.paintChip_C" _returnvalue_4 "AlwaysSpawn" "OverrideRootScale" null (`KismetMathLibrary.FFloor` (* _output_get _luckmulti)) null)
      (while (>= _currentchips 1)
        (`/Engine/EditorBlueprintResources/StandardMacros.DecrementInt` _currentchips))
      (if (<= (`KismetMathLibrary.RandomFloatInRange` 0.0 100.0) (`KismetMathLibrary.Conv_IntToDouble` (* _currentchips 100)))
        (`|SpawnActorFromClass` "/Game/Blueprints/paintChip.paintChip_C" _returnvalue_4 "Undefined" "OverrideRootScale" null 1 null)))
    (:`then_1`
      (bind _asmy_game_2 (cast `/Game/Blueprints/MyGame` (`GameplayStatics.GetGameInstance`)))
      ;[1 1 1] Spawn Coins
      (bind _coinmulti (`/Game/Blueprints/MyGame.getCoinMulti` _asmy_game_2))
      (`|SpawnActorFromClass` "/Game/Blueprints/Coin.Coin_C" (`KismetMathLibrary.MakeTransform` _returnvalue_2 _returnvalue_3 (0.2 0.05 0.2)) "AlwaysSpawn" "OverrideRootScale" null (`KismetMathLibrary.FTrunc` (* (`KismetMathLibrary.RandomIntegerInRange` 50 75) _coinmulti)) null))
    (:`then_2`
      ;[1 1 1] Item drop table
      (bind _dropmulti (`/Game/Blueprints/MyGame.getDropMulti` (`self.As My Game`) :!label _label))
      (if (< _counter 6)
        (`|SpawnActorFromClass` (select `int` (`KismetMathLibrary.RandomIntegerInRange` 0 4) :`0` "/Game/Blueprints/speedPickup.speedPickup_C" :`1` "/Game/Blueprints/lightAmmoDrop.lightAmmoDrop_C" :`2` "/Game/Blueprints/grenadeDrop.grenadeDrop_C" :`3` "/Game/Blueprints/heavyAmmoDrop.heavyAmmoDrop_C" :`4` "/Game/Blueprints/healthPackDrop.healthPackDrop_C" :!type "Actor Class Reference") (`KismetMathLibrary.MakeTransform` _returnvalue_2 _returnvalue_3) "AdjustIfPossibleButAlwaysSpawn" "OverrideRootScale" null null) ; PIckup drop table
        (`/Engine/EditorBlueprintResources/StandardMacros.IncrementInt` _counter
          (:`  `
            (goto _label)))))
    (:`then_3`
      (`/Game/Blueprints/MyGame.getDropMulti` (`self.As My Game`)))
    (:`then_4`
      ;[1 1 1] Attachment drop table
      (if (< (`self.attachmentsSpawned`) 5) :!label _label_2
        (if (> _returnvalue 35.0)
          (if (> _returnvalue 55.0)
            (if (> _returnvalue 75.0)
              (if (> _returnvalue 90.0)
                (set `self.dropIndex` 4)
                (else
                  (set `self.dropIndex` 3)))
              (else
                (set `self.dropIndex` 2)))
            (else
              (set `self.dropIndex` 1)))
          (else
            (set `self.dropIndex` 0)))
        (`|SpawnActorFromClass` (select `int` (`self.dropIndex`) :`0` "/Game/Blueprints/AttachmentsAssets/commonAttachmentPickup.commonAttachmentPickup_C" :`1` "/Game/Blueprints/AttachmentsAssets/uncommonAttachmentPickup.uncommonAttachmentPickup_C" :`2` "/Game/Blueprints/AttachmentsAssets/rareAttachmentPickup.rareAttachmentPickup_C" :`3` "/Game/Blueprints/AttachmentsAssets/epicAttachmentPickup.epicAttachmentPickup_C" :`4` "/Game/Blueprints/AttachmentsAssets/legendaryAttachmentPickup.legendaryAttachmentPickup_C" :!type "Actor Class Reference") (`KismetMathLibrary.MakeTransform` _returnvalue_2 _returnvalue_3 (0.5 0.5 0.5)) "AdjustIfPossibleButAlwaysSpawn" "OverrideRootScale" null null) ; Attachment drop table
        (`/Engine/EditorBlueprintResources/StandardMacros.IncrementInt` (`self.attachmentsSpawned`)
          (:`  `
            (goto _label_2)))))))

(fn `ShootLeftBarrel`
  (`|SpawnActorFromClass` "/Game/Blueprints/BossProjectileBP.BossProjectileBP_C" (`SceneComponent.K2_GetComponentToWorld` (`self.LBarrel`)) "Undefined" "OverrideRootScale" self self)
  (`GameplayStatics.PlaySoundAtLocation` "/Game/FirstPerson/Audio/FirstPersonTemplateWeaponFire02.FirstPersonTemplateWeaponFire02" (0.0 0.0 0.0) (struct) 0.3 0.5 0.0 "/Game/Blueprints/BossProjAttennuation.BossProjAttennuation" null null))

(fn `ShootRightBarrel`
  (`|SpawnActorFromClass` "/Game/Blueprints/BossProjectileBP.BossProjectileBP_C" (`SceneComponent.K2_GetComponentToWorld` (`self.RBarrel`)) "Undefined" "OverrideRootScale" null self)
  (`GameplayStatics.PlaySoundAtLocation` "/Game/FirstPerson/Audio/FirstPersonTemplateWeaponFire02.FirstPersonTemplateWeaponFire02" (0.0 0.0 0.0) (struct) 0.3 0.5 0.0 "/Game/Blueprints/BossProjAttennuation.BossProjAttennuation" null null))

(fn `UserConstructionScript`)