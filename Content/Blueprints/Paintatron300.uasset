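; Paintatron300 is an interactable actor that opens a paint shop UI when picked up.
; Its Pickup event creates a PaintChips widget with itself as the Shop reference, adds it to the viewport, shows the mouse cursor and switches input to UI only.
; CloseShop removes that widget, restores game-only input and hides the cursor.
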(event `/Game/Blueprints/pickupInterface.Pickup`
  (bind _returnvalue (`|CreateWidget` "/Game/Widget/PaintChipsWBP.PaintChipsWBP_C" null self))
  (set `self.paintShopWBP` _returnvalue)
  (`UserWidget.AddToViewport` _returnvalue 0)
  (set `PlayerController.bShowMouseCursor` true (`GameplayStatics.GetPlayerController` 0))
  (`WidgetBlueprintLibrary.SetInputMode_UIOnlyEx` (`GameplayStatics.GetPlayerController` 0) null))

(fn `Close Shop`
  (bind _returnvalue (`GameplayStatics.GetPlayerController` 0))
  (`Widget.RemoveFromParent` (`self.paintShopWBP`))
  (`WidgetBlueprintLibrary.SetInputMode_GameOnly` _returnvalue)
  (set `PlayerController.bShowMouseCursor` false _returnvalue))

(fn `UserConstructionScript`)