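; Key-locked door that the player's Pickup interaction raises or lowers.
; Tick polls the FirstPersonCharacter for the key and swaps the door's glow material between unlocked and locked.
; Pickup alternates through a FlipFlop, instantly offsetting the actor vertically when the key is held, otherwise calling the no-key prompt.
; The FlipFlop precedes the key check, so failed attempts also flip the direction of the next move.
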(event `self.ReceiveTick`
  (params (DeltaSeconds :type "Float (single-precision)"))
  (bind _asfirst_person_character (cast `/Game/FirstPersonBP/Blueprints/FirstPersonCharacter` (`GameplayStatics.GetPlayerCharacter` 0)))
  (bind _keyvalue (`/Game/FirstPersonBP/Blueprints/FirstPersonCharacter.ReturnKey` _asfirst_person_character))
  (if _keyvalue
    (`PrimitiveComponent.SetMaterial` (`self.Door`) 1 "/Game/Assets/DiningHall/DoorGlow.DoorGlow")
    (else
      (`PrimitiveComponent.SetMaterial` (`self.Door`) 1 "/Game/Assets/DiningHall/DoorGlowLock.DoorGlowLock"))))

(event `/Game/Blueprints/pickupInterface.Pickup`
  (`/Engine/EditorBlueprintResources/StandardMacros.FlipFlop`
    (:`A`
      (bind _asfirst_person_character (cast `/Game/FirstPersonBP/Blueprints/FirstPersonCharacter` (`GameplayStatics.GetPlayerCharacter` 0)))
      (bind _keyvalue (`/Game/FirstPersonBP/Blueprints/FirstPersonCharacter.ReturnKey` _asfirst_person_character))
      (if _keyvalue
        (`self.K2_SetActorRelativeLocation` (`KismetMathLibrary.MakeVector` (.x (`self.K2_GetActorLocation`)) (.y (`self.K2_GetActorLocation`)) (+ (.z (`self.K2_GetActorLocation`)) 244.0)))
        (else
          (`/Game/FirstPersonBP/Blueprints/FirstPersonCharacter.ShowHasNoKeyPrompt` (stale _asfirst_person_character_2) :!label _label))))
    (:`B`
      (bind _asfirst_person_character_2 (cast `/Game/FirstPersonBP/Blueprints/FirstPersonCharacter` (`GameplayStatics.GetPlayerCharacter` 0)))
      (bind _keyvalue_2 (`/Game/FirstPersonBP/Blueprints/FirstPersonCharacter.ReturnKey` _asfirst_person_character_2))
      (if _keyvalue_2
        (`self.K2_SetActorRelativeLocation` (`KismetMathLibrary.MakeVector` (.x (`self.K2_GetActorLocation`)) (.y (`self.K2_GetActorLocation`)) (+ (.z (`self.K2_GetActorLocation`)) -244.0)))
        (else
          (goto _label))))))

(fn `UserConstructionScript`)