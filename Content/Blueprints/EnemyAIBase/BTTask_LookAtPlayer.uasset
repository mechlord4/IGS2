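; Behavior tree task that instantly turns a Floater or Spoder enemy to face the player character.
; It casts the controlled pawn to FloaterBP, then SpoderBP, and snaps its root component to the full look-at rotation toward player 0.
; It finishes successfully after rotating, but never finishes for any other pawn type.
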(event `self.ReceiveExecuteAI`
  (params (OwnerController :type "AIController Object Reference") (ControlledPawn :type "Pawn Object Reference"))
  (bind _asfloater_bp (cast `/Game/Blueprints/FloaterBP` ControlledPawn)
    (:`then`
      (`SceneComponent.K2_SetWorldRotation` (`Actor.RootComponent` _asfloater_bp) (`KismetMathLibrary.FindLookAtRotation` (`SceneComponent.K2_GetComponentLocation` (`Actor.RootComponent` ControlledPawn)) (`SceneComponent.K2_GetComponentLocation` (`Actor.RootComponent` (`GameplayStatics.GetPlayerCharacter` 0)))) false false)
      (`self.FinishExecute` true))
    (:`CastFailed`
      (bind _asspoder_bp (cast `/Game/Blueprints/SpoderBP` ControlledPawn))
      (bind _rootcomponent (`Actor.RootComponent` _asspoder_bp))
      (`SceneComponent.K2_SetWorldRotation` _rootcomponent (`KismetMathLibrary.FindLookAtRotation` (`SceneComponent.K2_GetComponentLocation` _rootcomponent) (`SceneComponent.K2_GetComponentLocation` (`Actor.RootComponent` (`GameplayStatics.GetPlayerCharacter` 0)))) false false)
      (`self.FinishExecute` true))))