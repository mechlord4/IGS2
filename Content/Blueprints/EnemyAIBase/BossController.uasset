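; BossController is the AI controller for a boss enemy, running the BossBT behavior tree on BeginPlay.
; Its AI Perception updates react only to the FirstPersonCharacter and branch on sight, hearing or damage sense.
; Each branch writes the sensed state to a Blackboard flag, with hearing also storing the stimulus location as HeardLocation.
; Hearing and damage events also print debug messages.
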(event `self.ReceiveBeginPlay`
  (`self.RunBehaviorTree` "/Game/Blueprints/EnemyAIBase/BossBT.BossBT"))

(event `self.AIPerception.OnTargetPerceptionUpdated`
  (params (Actor :type "Actor Object Reference") (Stimulus :type "AIStimulus Structure"))
  (bind (_age _expirationage _strength _stimuluslocation _receiverlocation _tag _bsuccessfullysensed) (break `AIStimulus` Stimulus))
  (bind (_age_2 _expirationage_2 _strength_2 _stimuluslocation_2 _receiverlocation_2 _tag_2 _bsuccessfullysensed_2) (break `AIStimulus` Stimulus))
  (bind _returnvalue (`AIBlueprintHelperLibrary.GetBlackboard` null))
  (cast `/Game/FirstPersonBP/Blueprints/FirstPersonCharacter` Actor)
  (bind _returnvalue_2 (`AIPerceptionSystem.GetSenseClassForStimulus` Stimulus))
  (if (== _returnvalue_2 "/Script/AIModule.AISense_Sight")
    (`BlackboardComponent.SetValueAsBool` (`AIBlueprintHelperLibrary.GetBlackboard` null) "CanSeePlayer" _bsuccessfullysensed)
    (else
      (bind _returnvalue_3 (`AIPerceptionSystem.GetSenseClassForStimulus` Stimulus))
      (if (== _returnvalue_3 "/Script/AIModule.AISense_Hearing")
        (`KismetSystemLibrary.PrintString` "Heard Player")
        (`BlackboardComponent.SetValueAsBool` _returnvalue "CanHearPlayer" _bsuccessfullysensed_2)
        (`BlackboardComponent.SetValueAsVector` _returnvalue "HeardLocation" _stimuluslocation_2)
        (else
          (bind _returnvalue_4 (`AIPerceptionSystem.GetSenseClassForStimulus` Stimulus))
          (if (== _returnvalue_4 "/Script/AIModule.AISense_Damage")
            (`KismetSystemLibrary.PrintString` "Damaged by player")
            (`BlackboardComponent.SetValueAsBool` (`AIBlueprintHelperLibrary.GetBlackboard` null) "Damaged" _bsuccessfullysensed)))))))

(fn `UserConstructionScript`)