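; SpodderController is the AI controller for the Spodder enemy, running the SpoderBT behavior tree on BeginPlay.
; Perception updates are handled only for the FirstPersonCharacter and routed by sense class into blackboard keys.
; Sight sets CanSee, hearing sets HeardLocation and CanHear, and damage latches DamagedByPlayer to true without clearing it here.
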(event `self.ReceiveBeginPlay`
  (`self.RunBehaviorTree` "/Game/Blueprints/EnemyAIBase/SpoderBT.SpoderBT"))

(event `self.AIPerception.OnTargetPerceptionUpdated`
  (params (Actor :type "Actor Object Reference") (Stimulus :type "AIStimulus Structure"))
  (bind (_age _expirationage _strength _stimuluslocation _receiverlocation _tag _bsuccessfullysensed) (break `AIStimulus` Stimulus))
  (bind _returnvalue (`AIBlueprintHelperLibrary.GetBlackboard` null))
  (cast `/Game/FirstPersonBP/Blueprints/FirstPersonCharacter` Actor)
  (bind _returnvalue_2 (`AIPerceptionSystem.GetSenseClassForStimulus` Stimulus))
  (if (== _returnvalue_2 "/Script/AIModule.AISense_Sight")
    (`BlackboardComponent.SetValueAsBool` (`AIBlueprintHelperLibrary.GetBlackboard` null) "CanSee" (`.bSuccessfullySensed` (break `AIStimulus` Stimulus)))
    (else
      (bind _returnvalue_3 (`AIPerceptionSystem.GetSenseClassForStimulus` Stimulus))
      (if (== _returnvalue_3 "/Script/AIModule.AISense_Hearing")
        (`BlackboardComponent.SetValueAsVector` _returnvalue "HeardLocation" _stimuluslocation)
        (`BlackboardComponent.SetValueAsBool` _returnvalue "CanHear" _bsuccessfullysensed)
        (else
          (bind _returnvalue_4 (`AIPerceptionSystem.GetSenseClassForStimulus` Stimulus))
          (if (== _returnvalue_4 "/Script/AIModule.AISense_Damage")
            (`BlackboardComponent.SetValueAsBool` (`AIBlueprintHelperLibrary.GetBlackboard` null) "DamagedByPlayer" true)))))))

(fn `UserConstructionScript`)