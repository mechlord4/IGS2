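; Behavior Tree task that turns an enemy AI pawn toward the player and picks a location near them.
; On execute it instantly rotates the controlled pawn along the direction to player character 0.
; It then writes a random navigable point within a fixed radius of the player to a vector Blackboard key.
; It prints a debug string and always finishes successfully, without checking line of sight.
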(event `self.ReceiveExecuteAI`
  (params (OwnerController :type "AIController Object Reference") (ControlledPawn :type "Pawn Object Reference"))
  (bind _returnvalue (`Actor.K2_GetActorLocation` (`GameplayStatics.GetPlayerCharacter` 0)))
  (`Actor.K2_SetActorRotation` ControlledPawn (`KismetMathLibrary.Conv_VectorToRotator` (- _returnvalue (`Actor.K2_GetActorLocation` ControlledPawn))) false)
  (`KismetSystemLibrary.PrintString` "CanSeePlayer")
  (`BTFunctionLibrary.SetBlackboardValueAsVector` (`self.Vector`) (`NavigationSystemV1.K2_GetRandomLocationInNavigableRadius` _returnvalue 300.0 null null))
  (`self.FinishExecute` true))