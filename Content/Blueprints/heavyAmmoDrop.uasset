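; Heavy ammo drop pickup that refills the player's heavy weapon reserve.
; On spawn, its cube gets a random upward and sideways velocity impulse, always toward positive X and Y, so it pops out into the world.
; When a FirstPersonCharacter overlaps it, it grants a fixed amount of heavy ammo and destroys itself, or prints a message and stays if the reserve is already full.
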(event `self.ReceiveBeginPlay`
  (`PrimitiveComponent.AddImpulse` (`self.Cube`) (`KismetMathLibrary.MakeVector` (`KismetMathLibrary.RandomFloatInRange` 100.0 300.0) (`KismetMathLibrary.RandomFloatInRange` 100.0 300.0) (`KismetMathLibrary.RandomFloatInRange` 300.0 500.0)) "None" true))

(event `self.ReceiveActorBeginOverlap`
  (params (OtherActor :type "Actor Object Reference"))
  (bind _asfirst_person_character (cast `/Game/FirstPersonBP/Blueprints/FirstPersonCharacter` OtherActor))
  (if (>= (`/Game/FirstPersonBP/Blueprints/FirstPersonCharacter.heavyReserve` _asfirst_person_character) (`/Game/FirstPersonBP/Blueprints/FirstPersonCharacter.heavyReserveMax` _asfirst_person_character))
    (`KismetSystemLibrary.PrintString` "Cant pickup ammo, ammo is full")
    (else
      (`/Game/FirstPersonBP/Blueprints/FirstPersonCharacter.pickupHeavyAmmo` _asfirst_person_character 20)
      (`self.K2_DestroyActor`))))

(fn `UserConstructionScript`)