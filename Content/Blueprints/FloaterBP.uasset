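; Floater enemy, an AI-controlled actor that fires projectiles from left and right barrels and drops loot on death.
; Tick sets the CloseToPlayer blackboard key by player distance, and any damage reduces Health and sets LowHealth regardless of the remaining amount.
; At zero health it runs two independent drop rolls, a random supply pickup and an attachment whose rarity comes from nested chance checks, then destroys itself.
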(event `self.ReceiveTick`
  (params (DeltaSeconds :type "Float (single-precision)"))
  (bind _returnvalue (`AIBlueprintHelperLibrary.GetBlackboard` (`AIBlueprintHelperLibrary.GetAIController` self)))
  (if (<= (`KismetMathLibrary.Vector_Distance` (`SceneComponent.K2_GetComponentLocation` (`self.RootComponent`)) (`SceneComponent.K2_GetComponentLocation` (`Actor.RootComponent` (`GameplayStatics.GetPlayerCharacter` 0)))) 2500.0)
    (`BlackboardComponent.SetValueAsBool` _returnvalue "CloseToPlayer" true)
    (else
      (`BlackboardComponent.SetValueAsBool` _returnvalue "CloseToPlayer" false))))

(event `self.ReceiveAnyDamage`
  (params (Damage :type "Float (single-precision)") (DamageType :type "DamageType Object Reference") (InstigatedBy :type "Controller Object Reference") (DamageCauser :type "Actor Object Reference"))
  (bind _output_get (set `self.Health` (- (`self.Health`) Damage)))
  (if true
    (`BlackboardComponent.SetValueAsBool` (`AIBlueprintHelperLibrary.GetBlackboard` null) "LowHealth" true)
    (if (<= _output_get 0.0)
      (`self.DropPickUp`)
      (`self.K2_DestroyActor`))))

(fn `DropPickUp`
  (bind _returnvalue (`KismetMathLibrary.RandomFloatInRange` 0.0 100.0))
  (bind _returnvalue_2 (`SceneComponent.K2_GetComponentLocation` (`self.CapsuleComponent`)))
  (bind _returnvalue_3 (`KismetMathLibrary.MakeRotator` 0.0 0.0 (`KismetMathLibrary.RandomFloatInRange` 0.0 360.0)))
  (`|ExecutionSequence`
    (:`then_0`
      ;[1 1 1] Item drop table
      (if (>= (`KismetMathLibrary.RandomFloatInRange` 0.0 100.0) 50.0)
        (`|SpawnActorFromClass` (select `int` (`KismetMathLibrary.RandomIntegerInRange` 0 4) :`0` "/Game/Blueprints/speedPickup.speedPickup_C" :`1` "/Game/Blueprints/lightAmmoDrop.lightAmmoDrop_C" :`2` "/Game/Blueprints/grenadeDrop.grenadeDrop_C" :`3` "/Game/Blueprints/heavyAmmoDrop.heavyAmmoDrop_C" :`4` "/Game/Blueprints/healthPackDrop.healthPackDrop_C" :!type "Actor Class Reference") (`KismetMathLibrary.MakeTransform` _returnvalue_2 _returnvalue_3) "Undefined" "OverrideRootScale" null null) ; PIckup drop table
      ))
    (:`then_1`
      ;[1 1 1] Attachment drop table
      (if (<= (`KismetMathLibrary.RandomFloatInRange` 0.0 100.0) 75.0)
        (if (> _returnvalue 30.0)
          (if (> _returnvalue 55.0)
            (if (> _returnvalue 75.0)
              (if (> _returnvalue 90.0)
                (set `self.dropIndex` 4)
                (else
                  (set `self.dropIndex` 3)))
              (else
                (set `self.dropIndex` 2)))
            (else
              (set `self.dropIndex` 1)))
          (else
            (set `self.dropIndex` 0)))
        (`|SpawnActorFromClass` (select `int` (`self.dropIndex`) :`0` "/Game/Blueprints/AttachmentsAssets/commonAttachmentPickup.commonAttachmentPickup_C" :`1` "/Game/Blueprints/AttachmentsAssets/uncommonAttachmentPickup.uncommonAttachmentPickup_C" :`2` "/Game/Blueprints/AttachmentsAssets/rareAttachmentPickup.rareAttachmentPickup_C" :`3` "/Game/Blueprints/AttachmentsAssets/epicAttachmentPickup.epicAttachmentPickup_C" :`4` "/Game/Blueprints/AttachmentsAssets/legendaryAttachmentPickup.legendaryAttachmentPickup_C" :!type "Actor Class Reference") (`KismetMathLibrary.MakeTransform` _returnvalue_2 _returnvalue_3 (0.5 0.5 0.5)) "AdjustIfPossibleButAlwaysSpawn" "OverrideRootScale" null null) ; Attachment drop table
      ))))

(fn `ShootLeftBarrel`
  (`|SpawnActorFromClass` "/Game/Blueprints/FloaterProjectileBP.FloaterProjectileBP_C" (`SceneComponent.K2_GetComponentToWorld` (`self.LBarrel`)) "Undefined" "OverrideRootScale" null null))

(fn `ShootRightBarrel`
  (`|SpawnActorFromClass` "/Game/Blueprints/FloaterProjectileBP.FloaterProjectileBP_C" (`SceneComponent.K2_GetComponentToWorld` (`self.RBarrel`)) "Undefined" "OverrideRootScale" null null))

(fn `UserConstructionScript`)