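; Paint chip pickup actor that flies toward the player and adds to their paint chip count.
; Overlap by the player character starts the Attraction timeline, which lerps the chip between the first-person character's mesh and its own current location using a normalized distance track.
; When the timeline finishes, it adds its chip amount to the MyGame game instance and destroys itself.
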(event `self.ReceiveActorBeginOverlap`
  (params (OtherActor :type "Actor Object Reference"))
  (if (== OtherActor (`GameplayStatics.GetPlayerCharacter` 0))
    (bind _asfirst_person_character (cast `/Game/FirstPersonBP/Blueprints/FirstPersonCharacter` OtherActor))
    (bind (_direction _distance_normalized_) (`Timeline|Attraction`)
      (:`Update`
        (`SceneComponent.K2_SetWorldLocation` (`self.PaintChip`) (`KismetMathLibrary.VLerp` (`SceneComponent.K2_GetComponentLocation` (`Character.Mesh` _asfirst_person_character)) (`SceneComponent.K2_GetComponentLocation` (`self.PaintChip`)) _distance_normalized_) false false))
      (:`Finished`
        (bind _asmy_game (cast `/Game/Blueprints/MyGame` (`GameplayStatics.GetGameInstance`)))
        (`/Game/Blueprints/MyGame.addPaintChips` _asmy_game (`self.numofChips`))
        (`self.K2_DestroyActor`)))))

(fn `UserConstructionScript`)