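; Shop actor that sells randomly rolled weapon attachments and ammo through a ShopWBP widget opened on Pickup.
; BeginPlay fills four slots with price, name and a pickup pre-spawned far off-map: three roll attachment rarity through nested random checks, slot 3 rolls heavy or light ammo.
; Getters expose each slot, GetSpawnItemLocation returns a jittered spawn transform, and Pickup and CloseShop toggle cursor and UI-only input.
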(event `self.ReceiveBeginPlay`
  (`self.Set Slot 1`)
  (`self.SetSlot2`)
  (`self.SetSlot3`)
  (`self.SetSlot4`))

(event `/Game/Blueprints/pickupInterface.Pickup`
  (bind _returnvalue (`|CreateWidget` "/Game/Widget/ShopWBP.ShopWBP_C" null self))
  (set `self.ShopWidget` _returnvalue)
  (`UserWidget.AddToViewport` _returnvalue 0)
  (set `PlayerController.bShowMouseCursor` true (`GameplayStatics.GetPlayerController` 0))
  (`WidgetBlueprintLibrary.SetInputMode_UIOnlyEx` (`GameplayStatics.GetPlayerController` 0) null))

(fn `CloseShop`
  (bind _returnvalue (`GameplayStatics.GetPlayerController` 0))
  (`Widget.RemoveFromParent` (`self.ShopWidget`))
  (`WidgetBlueprintLibrary.SetInputMode_GameOnly` _returnvalue)
  (set `PlayerController.bShowMouseCursor` false _returnvalue))

(fn `getSlot1Item`
  (returns (Actor :type "Actor Object Reference"))
  (return (`self.Slot1`)))

(fn `GetSlot1Name`
  (returns (Name :type String))
  (return (`self.Slot 1 Name`)))

(fn `GetSlot1Price`
  (returns (Price :type Integer))
  (return (`self.Slot 1 Price`)))

(fn `getSlot2Item`
  (returns (Actor :type "Actor Object Reference"))
  (return (`self.Slot2`)))

(fn `GetSlot2Name`
  (returns (Name :type String))
  (return (`self.Slot 2 Name`)))

(fn `GetSlot2Price`
  (returns (Price :type Integer))
  (return (`self.Slot 2 Price`)))

(fn `getSlot3Item`
  (returns (Slot3 :type "Actor Object Reference"))
  (return (`self.Slot3`)))

(fn `GetSlot3Name`
  (returns (Name :type String))
  (return (`self.Slot 3 Name`)))

(fn `GetSlot3Price`
  (returns (Price :type Integer))
  (return (`self.Slot 3 Price`)))

(fn `GetSlot4Item`
  (returns (`SLot 4` :type "Actor Object Reference"))
  (return (`self.Slot 4`)))

(fn `GetSlot4Name`
  (returns (Name :type String))
  (return (`self.Slot 4 Name`)))

(fn `GetSlot4Price`
  (returns (Price :type Integer))
  (return (`self.Slot 4 Price`)))

(fn `getSpawnItemLocation`
  (returns (NewParam :type "Transform Structure"))
  (bind _returnvalue (`KismetMathLibrary.RandomFloatInRange` -10.0 10.0))
  (bind _returnvalue_2 (`SceneComponent.K2_GetComponentToWorld` (`self.Spawn item location`)))
  (return (`KismetMathLibrary.MakeTransform` (`KismetMathLibrary.MakeVector` (+ (.x (.location _returnvalue_2)) _returnvalue) (+ (.y (.location _returnvalue_2)) _returnvalue) (+ (.z (.location _returnvalue_2)) _returnvalue)) (.rotation _returnvalue_2) (.scale _returnvalue_2))))

(fn `Set Slot 1`
  (bind _returnvalue (`KismetMathLibrary.RandomIntegerInRange` 0 100))
  (if (> _returnvalue 30)
    (if (> _returnvalue 50)
      (if (> _returnvalue 70)
        (if (> _returnvalue 90)
          (set `self.AttachmentIndex` 4)
          (set `self.Slot 1 Price` (`KismetMathLibrary.RandomIntegerInRange` 70 100))
          (set `self.Slot 1 Name` "Legendary Attachment")
          (else
            (set `self.AttachmentIndex` 3)
            (set `self.Slot 1 Price` (`KismetMathLibrary.RandomIntegerInRange` 60 85))
            (set `self.Slot 1 Name` "Epic Attachment")))
        (else
          (set `self.AttachmentIndex` 2)
          (set `self.Slot 1 Price` (`KismetMathLibrary.RandomIntegerInRange` 45 65))
          (set `self.Slot 1 Name` "Rare Attachment")))
      (else
        (set `self.AttachmentIndex` 1)
        (set `self.Slot 1 Price` (`KismetMathLibrary.RandomIntegerInRange` 30 50))
        (set `self.Slot 1 Name` "Uncommon Attachment")))
    (else
      (set `self.AttachmentIndex` 0)
      (set `self.Slot 1 Price` (`KismetMathLibrary.RandomIntegerInRange` 15 35))
      (set `self.Slot 1 Name` "Common Attachment")))
  (bind _returnvalue_2 (`|SpawnActorFromClass` (select `int` (`self.AttachmentIndex`) :`0` "/Game/Blueprints/AttachmentsAssets/commonAttachmentPickup.commonAttachmentPickup_C" :`1` "/Game/Blueprints/AttachmentsAssets/uncommonAttachmentPickup.uncommonAttachmentPickup_C" :`2` "/Game/Blueprints/AttachmentsAssets/rareAttachmentPickup.rareAttachmentPickup_C" :`3` "/Game/Blueprints/AttachmentsAssets/epicAttachmentPickup.epicAttachmentPickup_C" :`4` "/Game/Blueprints/AttachmentsAssets/legendaryAttachmentPickup.legendaryAttachmentPickup_C" :!type "Actor Class Reference") (`KismetMathLibrary.MakeTransform` (-1000.0 -1000.0 -1000.0)) "Undefined" "OverrideRootScale" null null))
  (set `self.Slot1` _returnvalue_2))

(fn `SetSlot2`
  (bind _returnvalue (`KismetMathLibrary.RandomIntegerInRange` 0 100))
  (if (> _returnvalue 30)
    (if (> _returnvalue 50)
      (if (> _returnvalue 70)
        (if (> _returnvalue 90)
          (set `self.AttachmentIndex` 4)
          (set `self.Slot 2 Price` (`KismetMathLibrary.RandomIntegerInRange` 70 100))
          (set `self.Slot 2 Name` "Legendary Attachment")
          (else
            (set `self.AttachmentIndex` 3)
            (set `self.Slot 2 Price` (`KismetMathLibrary.RandomIntegerInRange` 60 85))
            (set `self.Slot 2 Name` "Epic Attachment")))
        (else
          (set `self.AttachmentIndex` 2)
          (set `self.Slot 2 Price` (`KismetMathLibrary.RandomIntegerInRange` 45 65))
          (set `self.Slot 2 Name` "Rare Attachment")))
      (else
        (set `self.AttachmentIndex` 1)
        (set `self.Slot 2 Price` (`KismetMathLibrary.RandomIntegerInRange` 30 50))
        (set `self.Slot 2 Name` "Uncommon Attachment")))
    (else
      (set `self.AttachmentIndex` 0)
      (set `self.Slot 2 Price` (`KismetMathLibrary.RandomIntegerInRange` 15 35))
      (set `self.Slot 2 Name` "Common Attachment")))
  (bind _returnvalue_2 (`|SpawnActorFromClass` (select `int` (`self.AttachmentIndex`) :`0` "/Game/Blueprints/AttachmentsAssets/commonAttachmentPickup.commonAttachmentPickup_C" :`1` "/Game/Blueprints/AttachmentsAssets/uncommonAttachmentPickup.uncommonAttachmentPickup_C" :`2` "/Game/Blueprints/AttachmentsAssets/rareAttachmentPickup.rareAttachmentPickup_C" :`3` "/Game/Blueprints/AttachmentsAssets/epicAttachmentPickup.epicAttachmentPickup_C" :`4` "/Game/Blueprints/AttachmentsAssets/legendaryAttachmentPickup.legendaryAttachmentPickup_C" :!type "Actor Class Reference") (`KismetMathLibrary.MakeTransform` (-1000.0 -1000.0 -1000.0)) "Undefined" "OverrideRootScale" null null))
  (set `self.Slot2` _returnvalue_2))

(fn `SetSlot3`
  (if (>= (`KismetMathLibrary.RandomIntegerInRange` 0 100) 45)
    (set `self.AmmoIndex` 1)
    (set `self.Slot 3 Price` 20)
    (set `self.Slot 3 Name` "Light Ammo")
    (else
      (set `self.AmmoIndex` 0)
      (set `self.Slot 3 Price` 30)
      (set `self.Slot 3 Name` "Heavy Ammo")))
  (bind _returnvalue (`|SpawnActorFromClass` (select `int` (`self.AmmoIndex`) :`0` "/Game/Blueprints/heavyAmmoDrop.heavyAmmoDrop_C" :`1` "/Game/Blueprints/lightAmmoDrop.lightAmmoDrop_C" :!type "Actor Class Reference") (`KismetMathLibrary.MakeTransform` (-1000.0 -1000.0 -1000.0)) "Undefined" "OverrideRootScale" null null))
  (set `self.Slot3` _returnvalue))

(fn `SetSlot4`
  (bind _returnvalue (`KismetMathLibrary.RandomIntegerInRange` 0 100))
  (if (> _returnvalue 30)
    (if (> _returnvalue 50)
      (if (> _returnvalue 70)
        (if (> _returnvalue 90)
          (set `self.AttachmentIndex` 4)
          (set `self.Slot 4 Price` (`KismetMathLibrary.RandomIntegerInRange` 70 100))
          (set `self.Slot 4 Name` "Legendary Attackment")
          (else
            (set `self.AttachmentIndex` 3)
            (set `self.Slot 4 Price` (`KismetMathLibrary.RandomIntegerInRange` 60 85))
            (set `self.Slot 4 Name` "Epic Attachment")))
        (else
          (set `self.AttachmentIndex` 2)
          (set `self.Slot 4 Price` (`KismetMathLibrary.RandomIntegerInRange` 45 65))
          (set `self.Slot 4 Name` "Rare Attachment")))
      (else
        (set `self.AttachmentIndex` 1)
        (set `self.Slot 4 Price` (`KismetMathLibrary.RandomIntegerInRange` 30 50))
        (set `self.Slot 4 Name` "Uncommon Attachment")))
    (else
      (set `self.AttachmentIndex` 0)
      (set `self.Slot 4 Price` (`KismetMathLibrary.RandomIntegerInRange` 15 35))
      (set `self.Slot 4 Name` "Common Attachment")))
  (bind _returnvalue_2 (`|SpawnActorFromClass` (select `int` (`self.AttachmentIndex`) :`0` "/Game/Blueprints/AttachmentsAssets/commonAttachmentPickup.commonAttachmentPickup_C" :`1` "/Game/Blueprints/AttachmentsAssets/uncommonAttachmentPickup.uncommonAttachmentPickup_C" :`2` "/Game/Blueprints/AttachmentsAssets/rareAttachmentPickup.rareAttachmentPickup_C" :`3` "/Game/Blueprints/AttachmentsAssets/epicAttachmentPickup.epicAttachmentPickup_C" :`4` "/Game/Blueprints/AttachmentsAssets/legendaryAttachmentPickup.legendaryAttachmentPickup_C" :!type "Actor Class Reference") (`KismetMathLibrary.MakeTransform` (-1000.0 -1000.0 -1000.0)) "Undefined" "OverrideRootScale" null null))
  (set `self.Slot 4` _returnvalue_2))

(fn `UserConstructionScript`)