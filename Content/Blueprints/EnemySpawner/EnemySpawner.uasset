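; Enemy spawner actor that registers with the first EnemySpawnManagerBP on BeginPlay and spawns AI enemies at its root component's transform.
; StartSpawningEnemies adds the requested count to the pending total and calls a delayed loop that spawns one enemy per second until none remain.
; A random roll selects floater or spoder with matching behavior trees, but its threshold currently makes every spawn a spoder.
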(event `self.ReceiveBeginPlay`
  (bind _outactors (`GameplayStatics.GetAllActorsOfClass` "/Game/Blueprints/EnemySpawner/EnemySpawnManagerBP.EnemySpawnManagerBP_C"))
  (`/Game/Blueprints/EnemySpawner/EnemySpawnManagerBP.addToEnemySpawnerArray` (`|GetArrayItem` _outactors) self))

(event `self.ReceiveTick`
  (params (DeltaSeconds :type "Float (single-precision)")))

(event `spawnEnemyLoop`
  (bind (_returnvalue_location _returnvalue_rotation) (`KismetMathLibrary.BreakTransform` (`SceneComponent.K2_GetComponentToWorld` (`self.DefaultSceneRoot`))))
  (if (> (`self.enemiesToSpawn`) 0) :!label _label
    (`/Engine/EditorBlueprintResources/StandardMacros.DecrementInt` (`self.enemiesToSpawn`)
      (:`  `
        (if (< (`KismetMathLibrary.RandomIntegerInRange` 0 100) 0)
          (`AIBlueprintHelperLibrary.SpawnAIFromClass` "/Game/Blueprints/FloaterBP.FloaterBP_C" "/Game/Blueprints/EnemyAIBase/EnemyBT.EnemyBT" _returnvalue_location _returnvalue_rotation true null)
          (else
            (`AIBlueprintHelperLibrary.SpawnAIFromClass` "/Game/Blueprints/SpoderBP.SpoderBP_C" "/Game/Blueprints/EnemyAIBase/SpoderBT.SpoderBT" _returnvalue_location _returnvalue_rotation true null)))
        (`KismetSystemLibrary.Delay` 1.0)
        (goto _label)))))

(fn `startSpawningEnemies`
  (params (enemyNum :type Integer))
  (set `self.enemiesToSpawn` (+ enemyNum (`self.enemiesToSpawn`)))
  (`self.spawnEnemyLoop`))

(fn `UserConstructionScript`)