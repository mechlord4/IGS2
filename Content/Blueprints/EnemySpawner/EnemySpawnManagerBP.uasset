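; Manager for endless-mode enemy waves, which shows the endless HUD on the first-person character at BeginPlay.
; Each externally triggered wave increases the enemy total linearly with wave number and updates the HUD count.
; After a short delay, it repeatedly hands random batches of up to three enemies to random registered spawners until none remain.
; Helper functions register spawners and adjust the wave's enemy count.
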(event `startEndlessMode`
  (bind _asfirst_person_character (cast `/Game/FirstPersonBP/Blueprints/FirstPersonCharacter` (`GameplayStatics.GetPlayerCharacter` 0)))
  (`/Game/FirstPersonBP/Blueprints/FirstPersonCharacter.showEndlessModeHud` _asfirst_person_character))

(event `self.ReceiveBeginPlay`
  (`self.startEndlessMode`))

(event `self.ReceiveTick`
  (params (DeltaSeconds :type "Float (single-precision)")))

(event `startNextWave`
  (bind _enemywavetotal (`self.enemyWaveTotal`))
  (`/Engine/EditorBlueprintResources/StandardMacros.IncrementInt` (`self.currentWave`)
    (:`  `
      (set `self.enemyWaveTotal` (`KismetMathLibrary.FTrunc` (+ (* (`KismetMathLibrary.Conv_IntToDouble` (`self.currentWave`)) 2.15) 3.0)))
      (bind _asfirst_person_character (cast `/Game/FirstPersonBP/Blueprints/FirstPersonCharacter` (`GameplayStatics.GetPlayerCharacter` 0)))
      (`/Game/FirstPersonBP/Blueprints/FirstPersonCharacter.Update Endless Enemies Left Alive` _asfirst_person_character _enemywavetotal)
      (set `self.enemiesLeftToSpawn` _enemywavetotal)
      (`KismetSystemLibrary.Delay` 3.0)
      (bind _asenemy_spawner (cast `/Game/Blueprints/EnemySpawner/EnemySpawner` (`|GetArrayItem` (`self.enemySpawnerArray`) (`KismetMathLibrary.RandomIntegerInRange` 0 (- (`KismetArrayLibrary.Array_Length` (`self.enemySpawnerArray`)) 1))) :!label _label))
      (if (>= (`self.enemiesLeftToSpawn`) 3)
        (bind _output_get (set `self.randomEnemiesToSpawn` (`KismetMathLibrary.RandomIntegerInRange` 1 3)))
        (`/Game/Blueprints/EnemySpawner/EnemySpawner.startSpawningEnemies` _asenemy_spawner _output_get)
        (set `self.enemiesLeftToSpawn` (- (`self.enemiesLeftToSpawn`) _output_get))
        (else
          (bind _output_get_2 (set `self.randomEnemiesToSpawn` (`KismetMathLibrary.RandomIntegerInRange` 1 (`self.enemiesLeftToSpawn`))))
          (`/Game/Blueprints/EnemySpawner/EnemySpawner.startSpawningEnemies` _asenemy_spawner _output_get_2)
          (set `self.enemiesLeftToSpawn` (- (`self.enemiesLeftToSpawn`) _output_get_2))))
      (if (> (`self.enemiesLeftToSpawn`) 0)
        (`KismetSystemLibrary.Delay` 1.0)
        (goto _label)))))

(fn `addToEnemySpawnerArray`
  (params (enemySpawner :type "Actor Object Reference"))
  (`KismetArrayLibrary.Array_Add` (`self.enemySpawnerArray`) enemySpawner))

(fn `decrementEnemiesLeft`
  (`/Engine/EditorBlueprintResources/StandardMacros.DecrementInt` (`self.enemyWaveTotal`)))

(fn `incrementEnemiesLeft`
  (`/Engine/EditorBlueprintResources/StandardMacros.IncrementInt` (`self.enemyWaveTotal`)))

(fn `UserConstructionScript`)