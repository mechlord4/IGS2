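; Spoder enemy character that feeds its AI Blackboard with player proximity and damage flags, and can self-destruct in an explosion.
; Reaching a nav link launches it toward the destination using ballistic velocity math.
; Explode sphere-traces for the player to apply impulse and damage, then spawns an effect and destroys the actor.
; Death by damage rolls two drop tables: random pickups and rarity-tiered attachments via nested chance checks.
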(event EventTick
  (params (DeltaSeconds :type Float%20%28single-precision%29))
  (bind _returnvalue (Utilities|Name|MakeLiteralName "CloseToPlayer"))
  (bind _self self)
  (bind _returnvalue_2 (AI|GetAIController _self))
  (bind _returnvalue_3 (AI|GetBlackboard _returnvalue_2))
  (if (<= (Math|Vector|Distance(Vector) (Transformation|GetWorldLocation (Variables|Transformation|GetRootComponent self)) (Transformation|GetWorldLocation (Variables|/Script/Engine.Actor|GetRootComponent (Game|GetPlayerCharacter 0)))) 5e+02)
    (AI|Components|Blackboard|SetValueasBool _returnvalue_3 _returnvalue true)
    (else
      (AI|Components|Blackboard|SetValueasBool _returnvalue_3 _returnvalue false))))

(event EventNavLinkReached
  (params (NavLinkDestination :type Vector :default "0, 0, 0"))
  (bind (_x _y _z) (Math|Vector|BreakVector NavLinkDestination))
  (bind _returnvalue (Transformation|GetActorLocation))
  (bind (_x_2 _y_2 _z_2) (Math|Vector|BreakVector _returnvalue))
  (Character|LaunchCharacter (Math|Vector|MakeVector (|((DestinationX-startX)/{B1EF43EF-4146-7726-7676-0DAE33789280}) _x _x_2) (|((DestinationY-StartY)/{B1EF43EF-4146-7726-7676-0DAE33789280}) _y _y_2) (|((DestinationHeight-(StartHeight-(((Power({B1EF43EF-4146-7726-7676-0DAE33789280},2))*0.500000)*{1D553B6C-462F-8A39-E75A-D0890AF5B60D})))/{B1EF43EF-4146-7726-7676-0DAE33789280}) _z _z_2)) false false))

(event Game|Damage|EventAnyDamage
  (params (Damage :type Float%20%28single-precision%29) (DamageType :type Damage%20Type%20Object%20Reference) (InstigatedBy :type Controller%20Object%20Reference) (DamageCauser :type Actor%20Object%20Reference))
  (bind _output_get (Variables|Default|SetHealth (- (Variables|Default|GetHealth) Damage)))
  (AI|Components|Blackboard|SetValueasBool (Variables|/Script/AIModule.AIController|GetBlackboard (AI|GetAIController self)) (Utilities|Name|MakeLiteralName "DamagedByPlayer") true)
  (if (<= _output_get 0.0)
    (CallFunction|DropPickUp)
    (Actor|DestroyActor)))

(fn ConstructionScript
  (Variables|Default|SetHealth 5e+01))

(fn Explode
  (bind _capsulecomponent (Variables|Collision|GetCapsuleComponent))
  (bind _returnvalue (Transformation|GetWorldLocation _capsulecomponent))
  (bind _outhits (Collision|MultiSphereTraceByChannel _returnvalue _returnvalue 6e+02 "TraceTypeQuery1" false 0 "Persistent"))
  (for _array_element _outhits
    (Development|PrintString (Utilities|GetDisplayName (.hitactor _array_element)))
    (if (== (.hitactor _array_element) "/Game/FirstPersonBP/Blueprints/FirstPersonCharacter.FirstPersonCharacter")
      (Class|RadialForceComponent|FireImpulse (Variables|Default|GetRadialForce))
      (Game|Damage|ApplyDamage 0 2e+01 0 self)
      (Effects|SpawnEmitteratLocation "/Game/StarterContent/Particles/P_Explosion.P_Explosion" (Transformation|GetWorldLocation (Variables|Collision|GetCapsuleComponent)) "0, 0, 0" "6.000000,6.000000,6.000000")
      (Actor|DestroyActor)))
  (Effects|SpawnEmitteratLocation "/Game/StarterContent/Particles/P_Explosion.P_Explosion" (Transformation|GetWorldLocation (Variables|Collision|GetCapsuleComponent)) "0, 0, 0" "6.000000,6.000000,6.000000")
  (Actor|DestroyActor))

(fn DropPickUp
  (bind _returnvalue (Math|Random|RandomFloatinRange 0.0 1e+02))
  (Utilities|FlowControl|Sequence
    (:then_0
      ;[1 1 1] Item drop table
      (if (>= (Math|Random|RandomFloatinRange 0.0 1e+02) 3e+01)
        (Game|SpawnActorfromClass (Utilities|Select :Index (Math|Random|RandomIntegerinRange 0 4) :Option%200 "/Game/Blueprints/speedPickup.speedPickup_C" :Option%201 "/Game/Blueprints/lightAmmoDrop.lightAmmoDrop_C" :Option%202 "/Game/Blueprints/grenadeDrop.grenadeDrop_C" :Option%203 "/Game/Blueprints/heavyAmmoDrop.heavyAmmoDrop_C" :Option%204 "/Game/Blueprints/healthPackDrop.healthPackDrop_C") (Math|Transform|MakeTransform (Transformation|GetWorldLocation (Variables|Collision|GetCapsuleComponent)) (Math|Rotator|MakeRotator 0.0 0.0 (Math|Random|RandomFloatinRange 0.0 3.6e+02))) "Undefined" 0 0) ; PIckup drop table
      ))
    (:then_1
      ;[1 1 1] Attachment drop table
      (if (<= (Math|Random|RandomFloatinRange 0.0 1e+02) 6e+01)
        (if (> _returnvalue 3e+01) ; check for uncommon
          (if (> _returnvalue 55.0) ; check for rare
            (if (> _returnvalue 75.0) ; check for epic
              (if (> _returnvalue 9e+01) ; check for legendary
                (Variables|Default|SetdropIndex 4)
                (else
                  (Variables|Default|SetdropIndex 3)))
              (else
                (Variables|Default|SetdropIndex 2)))
            (else
              (Variables|Default|SetdropIndex 1)))
          (else
            (Variables|Default|SetdropIndex 0)))
        (Game|SpawnActorfromClass (Utilities|Select :Index (Variables|Default|GetdropIndex) :Option%200 "/Game/Blueprints/AttachmentsAssets/commonAttachmentPickup.commonAttachmentPickup_C" :Option%201 "/Game/Blueprints/AttachmentsAssets/uncommonAttachmentPickup.uncommonAttachmentPickup_C" :Option%202 "/Game/Blueprints/AttachmentsAssets/rareAttachmentPickup.rareAttachmentPickup_C" :Option%203 "/Game/Blueprints/AttachmentsAssets/epicAttachmentPickup.epicAttachmentPickup_C" :Option%204 "/Game/Blueprints/AttachmentsAssets/legendaryAttachmentPickup.legendaryAttachmentPickup_C") (Math|Transform|MakeTransform "0, 0, 0" "0, 0, 0" "0.500000,0.500000,0.500000") "AdjustIfPossibleButAlwaysSpawn" 0 0) ; Attachment drop table
      ))))

(fn StopTree
  (AI|Components|Blackboard|SetValueasBool (Variables|/Script/AIModule.AIController|GetBlackboard (AI|GetAIController self)) (Utilities|Name|MakeLiteralName "isDone") true))