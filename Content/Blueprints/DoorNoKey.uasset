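; Door Blueprint that opens and closes vertically, with no key check in its logic.
; Each Pickup event drives a FlipFlop that alternately raises and lowers the actor by a fixed Z offset.
; The move is instant and unswept, computed from the actor's world location but applied through SetActorRelativeLocation, so it assumes an unattached actor.
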(event `/Game/Blueprints/pickupInterface.Pickup`
  (`/Engine/EditorBlueprintResources/StandardMacros.FlipFlop`
    (:`A`
      (`self.K2_SetActorRelativeLocation` (`KismetMathLibrary.MakeVector` (.x (`self.K2_GetActorLocation`)) (.y (`self.K2_GetActorLocation`)) (+ (.z (`self.K2_GetActorLocation`)) 244.0))))
    (:`B`
      (`self.K2_SetActorRelativeLocation` (`KismetMathLibrary.MakeVector` (.x (`self.K2_GetActorLocation`)) (.y (`self.K2_GetActorLocation`)) (+ (.z (`self.K2_GetActorLocation`)) -244.0))))))

(fn `UserConstructionScript`)