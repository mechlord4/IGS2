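; Weapon attachment pickup that permanently changes one random stat on the player's weapon, with only the Light weapon implemented so far.
; One second after BeginPlay it takes a random Light attribute from FirstPersonCharacter and prints debug text.
; Pickup halves fire rate or reload time and doubles other attributes, based on the value cached at spawn.
; It writes the result to the player's attribute array, refreshes attributes and damage, then destroys itself.
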(event `self.ReceiveBeginPlay`
  (`KismetSystemLibrary.Delay` 1.0) ; for testing reasons: player variables must be instantiated first so spawning it in scene would instantiate with empty variables
  (bind _asfirst_person_character (cast `/Game/FirstPersonBP/Blueprints/FirstPersonCharacter` (`GameplayStatics.GetPlayerCharacter` 0)))
  (bind _output_get (set `self.weaponType` (`KismetMathLibrary.RandomIntegerInRange` 0)))
  (switch `int` _output_get ; chooses what weapon the attachment is for
    (:`0`
      (bind (_attributename _attributevalue _arrayindex) (`/Game/FirstPersonBP/Blueprints/FirstPersonCharacter.getRandomLightAttribute` _asfirst_person_character))
      (`KismetSystemLibrary.PrintString` (`KismetStringLibrary.Conv_DoubleToString` _attributevalue))
      (`KismetSystemLibrary.PrintString` (`KismetStringLibrary.Conv_NameToString` _attributename))
      (`KismetSystemLibrary.PrintString` "added to")
      (`KismetSystemLibrary.PrintString` (`KismetStringLibrary.Conv_DoubleToString` (`self.PositiveStat1`)))
      (`KismetSystemLibrary.PrintString` "Positive percent of")
      (`KismetSystemLibrary.PrintString` "Light attachment dropped with:"))))

(event `/Game/Blueprints/pickupInterface.Pickup`
  (switch `int` (`KismetMathLibrary.RandomIntegerInRange` 0)
    (:`0`
      (bind _asfirst_person_character (cast `/Game/FirstPersonBP/Blueprints/FirstPersonCharacter` (`GameplayStatics.GetPlayerCharacter` 0)))
      (if (== (stale `self.ReceiveBeginPlay` _attributename) "Light Fire Rate")
        (`KismetArrayLibrary.Array_Set` (`/Game/FirstPersonBP/Blueprints/FirstPersonCharacter.lightAttributeValues` _asfirst_person_character) (stale `self.ReceiveBeginPlay` _arrayindex) (* (stale `self.ReceiveBeginPlay` _attributevalue) 0.5) :!label _label) ; If halving the value is a benefit
        (elif (== (stale `self.ReceiveBeginPlay` _attributename) "Light Reload Time")
          (goto _label)
          (else
            (`KismetArrayLibrary.Array_Set` (`/Game/FirstPersonBP/Blueprints/FirstPersonCharacter.lightAttributeValues` _asfirst_person_character) (stale `self.ReceiveBeginPlay` _arrayindex) (* (stale `self.ReceiveBeginPlay` _attributevalue) 2.0)) ; If increasing the value is a benefit
          )))
      (`/Game/FirstPersonBP/Blueprints/FirstPersonCharacter.setLightAttributes` _asfirst_person_character)
      (`/Game/FirstPersonBP/Blueprints/FirstPersonCharacter.calculateDamage` _asfirst_person_character)
      (`self.K2_DestroyActor`))))

(fn `UserConstructionScript`)