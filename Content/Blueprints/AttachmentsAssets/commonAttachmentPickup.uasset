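; Common weapon attachment pickup that grants the player a random percentage bonus to a Light or Heavy weapon attribute.
; BeginPlay rolls the stat and launches the cube, then after a delay non-drops pick weapon and attribute and pack an attachment struct.
; Pickup checks inventory space, adds the bonus, recalculates damage, stores itself and hides at origin.
; DropAttachment removes the bonus; SetValuesFromStruct loads saved values; overlap logic is unused.
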(event `self.ReceiveBeginPlay`
  ;[1 1 1] Attachment Spawn Sequence
  (`|ExecutionSequence`
    (:`then_0`
      (`KismetSystemLibrary.Delay` 1.0) ; for testing reasons: player variables must be instantiated first so spawning it in scene would instantiate with empty variables
      (if (not (`self.isADrop`))
        (bind _asfirst_person_character (cast `/Game/FirstPersonBP/Blueprints/FirstPersonCharacter` (`GameplayStatics.GetPlayerCharacter` 0)))
        (bind _output_get (set `self.weaponType` (`KismetMathLibrary.RandomIntegerInRange` 0 1)))
        (switch `int` _output_get ; chooses what weapon the attachment is for
          (:`0`
            ;[1 1 1] Light attachment spawn sequence
            (bind (_attributename _attributevalue _arrayindex) (`/Game/FirstPersonBP/Blueprints/FirstPersonCharacter.getRandomLightAttribute` _asfirst_person_character))
            (set `self.playerArrayIndex` _arrayindex)
            (`KismetSystemLibrary.PrintString` (`KismetStringLibrary.Concat_StrStr` "Light attachment dropped with: " "Positive percent of " (`KismetStringLibrary.Conv_DoubleToString` (`self.PositiveStat1`)) " added to " (`KismetStringLibrary.Conv_NameToString` _attributename))))
          (:`1`
            ;[1 1 1] Heavy attachment spawn sequence
            (bind (_attributename_2 _attributevalue_2 _arrayindex_2) (`/Game/FirstPersonBP/Blueprints/FirstPersonCharacter.getRandomHeavyAttribute` _asfirst_person_character))
            (set `self.playerArrayIndex` _arrayindex_2)
            (`KismetSystemLibrary.PrintString` (`KismetStringLibrary.Concat_StrStr` "Heavy attachment dropped with: " "Positive percent of " (`KismetStringLibrary.Conv_DoubleToString` (`self.PositiveStat1`)) " added to " (`KismetStringLibrary.Conv_NameToString` _attributename_2)))))
        (set `self.attachmentStruct` (make `/Game/Blueprints/AttachmentsAssets/attachmentStatsStruct` (`self.PositiveStat1`) (`self.NegativeStat1`) (`self.attachmentRarity`) (`self.weaponType`) (`self.playerArrayIndex`) true (struct :`R` 1.0 :`G` 1.0 :`B` 1.0 :`A` 1.0)))))
    (:`then_1`
      (set `self.PositiveStat1` (/ (`KismetMathLibrary.Conv_IntToDouble` (`KismetMathLibrary.RandomIntegerInRange` 50 150)) 10.0)))
    (:`then_2`
      (`PrimitiveComponent.AddImpulse` (`self.Cube`) (`KismetMathLibrary.MakeVector` (`KismetMathLibrary.RandomFloatInRange` -300.0 300.0) (`KismetMathLibrary.RandomFloatInRange` -300.0 300.0) (`KismetMathLibrary.RandomFloatInRange` 300.0 500.0)) "None" true))))

(event `/Game/Blueprints/pickupInterface.Pickup`
  (bind _playerarrayindex (`self.playerArrayIndex`))
  (bind _playerarrayindex_2 (`self.playerArrayIndex`))
  ;[1 1 1] Pickup attachment function
  (bind _asfirst_person_character (cast `/Game/FirstPersonBP/Blueprints/FirstPersonCharacter` (`GameplayStatics.GetPlayerCharacter` 0)))
  (bind _returnvalue (`KismetArrayLibrary.Array_Length` (`/Game/FirstPersonBP/Blueprints/FirstPersonCharacter.attachmentInventory` _asfirst_person_character)))
  (if (< (`KismetMathLibrary.Conv_IntToByte` _returnvalue) (`KismetMathLibrary.Conv_IntToByte` (`/Game/FirstPersonBP/Blueprints/FirstPersonCharacter.attachmentLimit` _asfirst_person_character)))
    (set `self.pickupSlot` (- _returnvalue 1))
    (switch `int` (`self.weaponType`)
      (:`0`
        (bind _lightattributeattachmentbonuses (`/Game/FirstPersonBP/Blueprints/FirstPersonCharacter.lightAttributeAttachmentBonuses` _asfirst_person_character))
        ;[1 1 1] Light attachment pickup function
        (`KismetArrayLibrary.Array_Set` _lightattributeattachmentbonuses _playerarrayindex_2 (+ (`|GetArrayItem` _lightattributeattachmentbonuses _playerarrayindex_2) (`self.PositiveStat1`)))
        (`/Game/FirstPersonBP/Blueprints/FirstPersonCharacter.calculateDamage` _asfirst_person_character)
        (`KismetSystemLibrary.PrintString` (`KismetStringLibrary.Conv_DoubleToString` (`|GetArrayItem` (`/Game/FirstPersonBP/Blueprints/FirstPersonCharacter.lightAttributeValues` _asfirst_person_character) _playerarrayindex_2)))
        (`KismetSystemLibrary.PrintString` "is now")
        (`KismetSystemLibrary.PrintString` (`KismetStringLibrary.Conv_NameToString` (stale `self.ReceiveBeginPlay` _attributename)))
        (`KismetSystemLibrary.PrintString` "Player just got benefits:")
        (`/Game/FirstPersonBP/Blueprints/FirstPersonCharacter.storeAttachment` _asfirst_person_character self)
        (`self.hideObjectAtOrigin`))
      (:`1`
        (bind _heavyattributeattachmentbonuses (`/Game/FirstPersonBP/Blueprints/FirstPersonCharacter.heavyAttributeAttachmentBonuses` _asfirst_person_character))
        ;[1 1 1] Heavy attachment pickup function
        (`KismetArrayLibrary.Array_Set` _heavyattributeattachmentbonuses _playerarrayindex (+ (`|GetArrayItem` _heavyattributeattachmentbonuses _playerarrayindex) (`self.PositiveStat1`)))
        (`/Game/FirstPersonBP/Blueprints/FirstPersonCharacter.calculateDamage` _asfirst_person_character)
        (`KismetSystemLibrary.PrintString` (`KismetStringLibrary.Conv_DoubleToString` (`|GetArrayItem` (`/Game/FirstPersonBP/Blueprints/FirstPersonCharacter.heavyAttributeValues` _asfirst_person_character) _playerarrayindex)))
        (`KismetSystemLibrary.PrintString` "is now")
        (`KismetSystemLibrary.PrintString` (`KismetStringLibrary.Conv_NameToString` (stale `self.ReceiveBeginPlay` _attributename_2)))
        (`KismetSystemLibrary.PrintString` "Player just got benefits:")
        (`/Game/FirstPersonBP/Blueprints/FirstPersonCharacter.storeAttachment` _asfirst_person_character self)
        (`self.hideObjectAtOrigin`)))
    (else
      (`KismetSystemLibrary.PrintString` "Player attachment inventory is full"))))

(event `Drop Attachment`
  (bind _playerarrayindex (`self.playerArrayIndex`))
  (bind _playerarrayindex_2 (`self.playerArrayIndex`))
  ;[1 1 1] Drop attachment system
  (set `self.pickupSlot` 0)
  (bind _asfirst_person_character (cast `/Game/FirstPersonBP/Blueprints/FirstPersonCharacter` (`GameplayStatics.GetPlayerCharacter` 0)))
  (switch `int` (`self.weaponType`)
    (:`0`
      (bind _lightattributeattachmentbonuses (`/Game/FirstPersonBP/Blueprints/FirstPersonCharacter.lightAttributeAttachmentBonuses` _asfirst_person_character))
      ;[1 1 1] Light attachment drop system
      (`KismetArrayLibrary.Array_Set` _lightattributeattachmentbonuses _playerarrayindex (- (`|GetArrayItem` _lightattributeattachmentbonuses _playerarrayindex) (`self.PositiveStat1`)))
      (`/Game/FirstPersonBP/Blueprints/FirstPersonCharacter.calculateDamage` _asfirst_person_character)
      (`KismetSystemLibrary.PrintString` (`KismetStringLibrary.Conv_DoubleToString` (`|GetArrayItem` (`/Game/FirstPersonBP/Blueprints/FirstPersonCharacter.lightAttributeValues` _asfirst_person_character) _playerarrayindex)))
      (`KismetSystemLibrary.PrintString` "is now")
      (`KismetSystemLibrary.PrintString` (`KismetStringLibrary.Conv_NameToString` (stale `self.ReceiveBeginPlay` _attributename)))
      (`KismetSystemLibrary.PrintString` "Player just lost benefits:"))
    (:`1`
      (bind _heavyattributeattachmentbonuses (`/Game/FirstPersonBP/Blueprints/FirstPersonCharacter.heavyAttributeAttachmentBonuses` _asfirst_person_character))
      ;[1 1 1] Heavy attachment drop system
      (`KismetArrayLibrary.Array_Set` _heavyattributeattachmentbonuses _playerarrayindex_2 (- (`|GetArrayItem` _heavyattributeattachmentbonuses _playerarrayindex_2) (`self.PositiveStat1`)))
      (`/Game/FirstPersonBP/Blueprints/FirstPersonCharacter.calculateDamage` _asfirst_person_character)
      (`KismetSystemLibrary.PrintString` (`KismetStringLibrary.Conv_DoubleToString` (`|GetArrayItem` (`/Game/FirstPersonBP/Blueprints/FirstPersonCharacter.heavyAttributeValues` _asfirst_person_character) _playerarrayindex_2)))
      (`KismetSystemLibrary.PrintString` "is now")
      (`KismetSystemLibrary.PrintString` (`KismetStringLibrary.Conv_NameToString` (stale `self.ReceiveBeginPlay` _attributename_2)))
      (`KismetSystemLibrary.PrintString` "Player just lost benefits:"))))

(event `self.ReceiveActorBeginOverlap`
  (params (OtherActor :type "Actor Object Reference"))
  ;[1 1 1] (unused) player interact overlap function (this has been moved to the first person character script
)

(event `self.ReceiveActorEndOverlap`
  (params (OtherActor :type "Actor Object Reference"))
  ;[1 1 1] (unused) player interact overlap function (this has been moved to the first person character script
)

(fn `hideObjectAtOrigin`
  (`self.K2_SetActorLocation` (0.0 0.0 0.0) false true)
  (`self.SetActorHiddenInGame` true)
  (`self.SetActorEnableCollision` false)
  (`PrimitiveComponent.SetSimulatePhysics` (`self.Cube`) false))

(fn `setValuesFromStruct`
  (params (attachmentStruct :type "/Game/Blueprints/AttachmentsAssets/attachmentStatsStruct Structure"))
  (set `self.PositiveStat1` attachmentStruct_PositiveStat1_2_C69FCE1B4E1DA21C9B6EF08B37316A81)
  (set `self.NegativeStat1` attachmentStruct_NegativeStat1_4_4C7919A64E7375D7E42DF19352954E85)
  (set `self.attachmentRarity` attachmentStruct_AttachmentRarity_9_83DF5FE54EE85B11DEA2FF85CCD6F1CD)
  (set `self.weaponType` attachmentStruct_WeaponType_11_FC61F9B64C2CC3A319EC5DB3AD8AD6C1)
  (set `self.playerArrayIndex` attachmentStruct_PlayerArrayIndex_13_3B38217340532E940B14EEBFBAB6FFC2)
  (set `self.isADrop` attachmentStruct_isADrop_16_73A80CDC42BB805418D81587B7BE0E50))

(fn `UserConstructionScript`)